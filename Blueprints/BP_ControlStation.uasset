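; Control station actor that opens an emissive-control UI when the player character steps into its collision.
; BeginPlay uses SetupMID to create dynamic M_Emissive_Master instances on mapped mesh slots, stored as Strong and Base sets with separate default power and a shared purple color.
; Overlap freezes movement and shows WBP_EmissiveControl, passing it a station reference, with UI-only input.
; End overlap restores walking and game input and removes the widget.
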(event `self.ReceiveBeginPlay`
  (bind _strongtargetmeshes (`self.StrongTargetMeshes`))
  (bind _basetargetmeshes (`self.BaseTargetMeshes`))
  ;[0.4825 0.224 1] Setup Strong DMIs
  (bind _keys (`BlueprintMapLibrary.Map_Keys` _strongtargetmeshes))
  (for _array_element _keys
    (`self.SetupMID` _array_element true (`BlueprintMapLibrary.Map_Find` _strongtargetmeshes _array_element)))
  ;[0.2718 0.2057 0.4072] Setup Base DMIs
  (bind _keys_2 (`BlueprintMapLibrary.Map_Keys` _basetargetmeshes))
  (for _array_element_2 _keys_2
    (`self.SetupMID` _array_element_2 false (`BlueprintMapLibrary.Map_Find` _basetargetmeshes _array_element_2))))

(event `self.CollisionComponent.OnComponentBeginOverlap`
  (params (OverlappedComponent :type "PrimitiveComponent Object Reference") (OtherActor :type "Actor Object Reference") (OtherComp :type "PrimitiveComponent Object Reference") (OtherBodyIndex :type Integer) (bFromSweep :type Boolean) (SweepResult :type "HitResult Structure (by ref)"))
  (bind _returnvalue (`GameplayStatics.GetPlayerController` 0))
  (bind _widgetref (`self.WidgetRef`))
  (bind _ashcharacter (cast `HCharacter` OtherActor))
  (`CharacterMovementComponent.SetMovementMode` (`Character.CharacterMovement` _ashcharacter) "MOVE_None" 0)
  (bind _returnvalue_2 (`|CreateWidget` "/Game/Addon_NS_Shell_ONE/UI/WBP_EmissiveControl.WBP_EmissiveControl_C" _returnvalue self))
  (set `self.WidgetRef` _returnvalue_2)
  (set `PlayerController.bShowMouseCursor` true _returnvalue)
  (`WidgetBlueprintLibrary.SetInputMode_UIOnlyEx` _returnvalue _widgetref)
  (`UserWidget.AddToViewport` _widgetref 0)
  (`UserWidget.PlayAnimation` _widgetref (`/Game/Addon_NS_Shell_ONE/UI/WBP_EmissiveControl.FadeIn` _widgetref) 0.0 1 "Forward" 1.0 false))

(event `self.CollisionComponent.OnComponentEndOverlap`
  (params (OverlappedComponent :type "PrimitiveComponent Object Reference") (OtherActor :type "Actor Object Reference") (OtherComp :type "PrimitiveComponent Object Reference") (OtherBodyIndex :type Integer))
  (bind _returnvalue (`GameplayStatics.GetPlayerController` 0))
  (bind _widgetref (`self.WidgetRef`))
  (bind _ashcharacter (cast `HCharacter` OtherActor))
  (`CharacterMovementComponent.SetMovementMode` (`Character.CharacterMovement` _ashcharacter) "MOVE_Walking" 0)
  (`Widget.RemoveFromParent` _widgetref)
  (set `PlayerController.bShowMouseCursor` false _returnvalue)
  (`WidgetBlueprintLibrary.SetInputMode_GameOnly` _returnvalue)
  (`UserWidget.PlayAnimation` _widgetref (`/Game/Addon_NS_Shell_ONE/UI/WBP_EmissiveControl.FadeOut` _widgetref) 0.0 1 "Forward" 1.0 false))

(fn `UserConstructionScript`)